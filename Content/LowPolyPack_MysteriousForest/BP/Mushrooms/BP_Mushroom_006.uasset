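; Mushroom prop from the low-poly Mysterious Forest pack, with separately tintable Foot and Hat components.
; The construction script creates dynamic material instances on slot 0 of each part and applies per-part base color, emissive intensity and emissive color from variables.
; Each of the three passes calls CreateDynamicMaterialInstance again before setting its parameter.
; The event graph holds only disabled stub events, so the actor has no runtime logic.
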(fn `UserConstructionScript`
  ;[1 1 1] Color Swap
  (bind _returnvalue (`PrimitiveComponent.CreateDynamicMaterialInstance` (`self.Foot`) 0 null "None"))
  (`MaterialInstanceDynamic.SetVectorParameterValue` _returnvalue "ColorParameter" (`self.Foot_`))
  (bind _returnvalue_2 (`PrimitiveComponent.CreateDynamicMaterialInstance` (`self.Hat`) 0 null "None"))
  (`MaterialInstanceDynamic.SetVectorParameterValue` _returnvalue_2 "ColorParameter" (`self.Hat_`))
  ;[1 1 1] Emissive Intensity
  (`PrimitiveComponent.CreateDynamicMaterialInstance` (`self.Foot`) 0 null "None")
  (`MeshComponent.SetScalarParameterValueOnMaterials` (`self.Foot`) "EmissiveParameter" (`self.Foot__`))
  (`PrimitiveComponent.CreateDynamicMaterialInstance` (`self.Hat`) 0 null "None")
  (`MeshComponent.SetScalarParameterValueOnMaterials` (`self.Hat`) "EmissiveParameter" (`self.Hat__`))
  ;[1 1 1] Emissive Color
  (bind _returnvalue_3 (`PrimitiveComponent.CreateDynamicMaterialInstance` (`self.Foot`) 0 null "None"))
  (`MaterialInstanceDynamic.SetVectorParameterValue` _returnvalue_3 "EmissiveColor" (`self.Foot_Color`))
  (bind _returnvalue_4 (`PrimitiveComponent.CreateDynamicMaterialInstance` (`self.Hat`) 0 null "None"))
  (`MaterialInstanceDynamic.SetVectorParameterValue` _returnvalue_4 "EmissiveColor" (`self.Hat_Color`)))