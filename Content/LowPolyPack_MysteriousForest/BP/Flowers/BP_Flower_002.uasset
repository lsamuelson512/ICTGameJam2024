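; Low-poly flower prop Blueprint from the Mysterious Forest pack, with separately colorable stem, leaf, flower and pistil parts.
; The Construction Script creates a dynamic material instance on the first material slot of each of the four components.
; It sets each one's ColorParameter from a matching color variable, so every placed instance can be tinted independently.
; The event graph holds only disabled default events, with no runtime logic.
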(fn `UserConstructionScript`
  (bind _returnvalue (`PrimitiveComponent.CreateDynamicMaterialInstance` (`self.Stem`) 0 null "None"))
  (`MaterialInstanceDynamic.SetVectorParameterValue` _returnvalue "ColorParameter" (`self.Stem_`))
  (bind _returnvalue_2 (`PrimitiveComponent.CreateDynamicMaterialInstance` (`self.Leaf`) 0 null "None"))
  (`MaterialInstanceDynamic.SetVectorParameterValue` _returnvalue_2 "ColorParameter" (`self.Leaf_`))
  (bind _returnvalue_3 (`PrimitiveComponent.CreateDynamicMaterialInstance` (`self.Flower`) 0 null "None"))
  (`MaterialInstanceDynamic.SetVectorParameterValue` _returnvalue_3 "ColorParameter" (`self.Flower_`))
  (bind _returnvalue_4 (`PrimitiveComponent.CreateDynamicMaterialInstance` (`self.Pistil`) 0 null "None"))
  (`MaterialInstanceDynamic.SetVectorParameterValue` _returnvalue_4 "ColorParameter" (`self.Pistil_`)))